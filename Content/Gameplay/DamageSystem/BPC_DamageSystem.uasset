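; Damage system component that tracks an owner's health, healing and death, with RepNotify state and event dispatchers for reactions.
; TakeDamage tests the instigator's yaw against a shield arc when blocking, then the CanBeDamaged macro routes to blocked, damaged or ignored.
; Damage applies headshot multipliers, then signals death or fires responses such as knock, stun and slow.
; Status effects, weakness/resistance and health getters are unfinished; an obsolete TakeDamage remains.
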(event EventBeginPlay)

(event EventTick
  (params (DeltaSeconds :type Float%20%28single-precision%29)))

(fn CHeal
  (params (Amount :type Integer))
  (if (not (Variables|Default|GetIsDead))
    (bind _output_get (Variables|Default|SetHealth (Math|Integer|Clamp(Integer) (+ Amount (Variables|Default|GetHealth)) 0 (Variables|Default|GetMaxHealth))))
    (return _output_get)))

(fn TakeDamage(OldDONTUSE)
  (params (DamageInfo :type S%20Damage%20Info%20Structure))
  (bind (_amount _headshotmultiplier _washeadshot _damagetype _damageelement _takestatuseffect _shoulddamageinvincible _canbeblocked _shouldforceinterrupt _canbeparried _hasdamageresponse _damageresponseinfo) (Utilities|Struct|BreakS_DamageInfo DamageInfo))
  (Development|PrintString "Taking Damage")
  (Utilities|CanbeDamaged false false false
    (:BlockDamage
      (Default|CallOnBlocked _canbeparried)
      (return false))
    (:DoDamage
      (Default|CallOnTakeDamage DamageInfo)
      (if true
        (bind _output_get (Variables|Default|SetHealth (Math|Integer|Clamp(Integer) (- (Variables|Default|GetHealth) _amount) -1 (Variables|Default|GetMaxHealth))))
        (if (<= _output_get 0)
          (Variables|Default|SetIsDead true)
          (Default|CallOnDeath)
          (return true)
          (elif _hasdamageresponse
            (CallFunction|TakeDamageResponse _damageresponseinfo)
            (return true)))))
    (:NoDamage
      (return false))))

(fn TakeDamageResponse
  (params (A_DamageResponseValues :type Array%20of%20S%20Damage%20Response%20Values%20Structures))
  (for _array_element A_DamageResponseValues
    (switch Utilities|FlowControl|Switch|SwitchonE_DamageResponse (.E_DamageResponse (Utilities|Struct|BreakS_DamageResponseValues _array_element))
      (:NewEnumerator1
        (Default|CallOnHitReaction _array_element))
      (:NewEnumerator2
        (Default|CallOnKnock _array_element)
        (Development|PrintString "Knocked"))
      (:NewEnumerator3
        (Default|CallOnStun _array_element))
      (:NewEnumerator4
        (Default|CallOnSlow _array_element))
      (:NewEnumerator5
        (Default|CallOnRoot _array_element))
      (:NewEnumerator6
        (Default|CallOnBlind _array_element)))))

(fn TakeStatusEffect
  (params (StatusEffect :type E_ElementalStatusEffect%20Enum :default "NewEnumerator0")))

(fn OnRepHealth
  (Default|CallOnHealthChange))

(fn OnRepMaxHealth)

(fn OnRepIsDead)

(fn CanTakeDamage
  (params (Location :type Vector))
  (bind _returnvalue (Components|GetOwner))
  (bind _shield_rotation (Variables|Default|GetShield%20Rotation))
  (bind _shield_rotation_delta (Variables|Default|GetShield%20Rotation%20Delta))
  (bind _returnvalue_2 (Math|Float|Absolute(Float) _shield_rotation_delta))
  (bind _yaw (Math|Rotator|BreakRotator _shield_rotation))
  (bind _returnvalue_3 (Transformation|GetActorLocation _returnvalue))
  (bind _returnvalue_4 (Math|Rotator|FindLookatRotation _returnvalue_3 Location))
  (bind _returnvalue_5 (+ _yaw _returnvalue_2))
  (bind _returnvalue_6 (- _yaw _returnvalue_2))
  (bind _returnvalue_7 (Math|Float|InRange(Float) (.yaw _returnvalue_4) _returnvalue_6 _returnvalue_5))
  (Development|PrintString (Utilities|String|ToString(Text) (Utilities|Text|FormatText "Comparing Base: {0}    Delta: {1}  Can Take Damage: {3}" _yaw _returnvalue_2 (not _returnvalue_7))) false false "(R=0.261077,G=1.000000,B=0.389478,A=1.000000)" 2e+01)
  (return _returnvalue_7))

(fn PlayerBlocking
  (params (Damage%20Info :type S%20Damage%20Info%20Structure))
  (bind _instigator (Utilities|Struct|BreakS_DamageInfo Damage%20Info))
  (Development|PrintString "Triggered try Block Damage" false false "(R=1.000000,G=0.061336,B=0.041440,A=1.000000)" 2e+01)
  (Utilities|IsValid _instigator
    (:Is%20Valid
      (bind _blockdamage (CallFunction|CanTakeDamage (Transformation|GetActorLocation _instigator)))
      (return _blockdamage))
    (:Is%20Not%20Valid
      (Development|PrintString "INVALID" false false "(R=0.910000,G=0.000000,B=0.000000,A=1.000000)" 2e+01))))

(fn DoDamage
  (params (B :type Integer))
  (bind _output_get (Variables|Default|SetHealth (Math|Integer|Clamp(Integer) (- (Variables|Default|GetHealth) B) -1 (Variables|Default|GetMaxHealth))))
  (return _output_get))

(fn GetCurrentHealth
  (return 0))

(fn GetMaxHealth
  (return 0))

(fn Heal
  (params (Amount :type Integer))
  (return 0))

(fn TakeDamage
  (params (DamageInfo :type S%20Damage%20Info%20Structure))
  (bind (_amount _headshotmultiplier _washeadshot _damagetype _damageelement _takestatuseffect _shoulddamageinvincible _canbeblocked _shouldforceinterrupt _canbeparried _hasdamageresponse _damageresponseinfo) (Utilities|Struct|BreakS_DamageInfo DamageInfo))
  (Development|PrintString "Recieving damage")
  (if (Variables|Default|GetIsBlocking)
    (bind _blockattack (CallFunction|PlayerBlocking DamageInfo)))
  ;[0.15 0.15 0.15 0.5] Macro to check for other Damage cases
  (Utilities|CanbeDamaged _shoulddamageinvincible _canbeblocked _blockattack
    (:BlockDamage
      ;[0.15 0.09961 0.1056 0.5] Blocked and Invinsible Responses
      (Default|CallOnBlocked _canbeparried DamageInfo)
      (return false))
    (:DoDamage
      ;[0.15 0.15 0.15 0.5] Check for weakness or resistances (NOT IMPLEMENTED JUST CHECKED FOR SCALABILITY
      (Default|CallOnTakeDamage DamageInfo)
      (if (not (Variables|Default|GetWeakness%20Or%20Resistant))
        ;[0.03311 0.15 0.04858 0.5] Set New Health and Check for Death
        (if (not _washeadshot)
          (bind _output_get (CallFunction|DoDamage _amount))
          (else
            (bind _output_get_2 (CallFunction|DoDamage (* _amount _headshotmultiplier)))))
        (Default|CallOnInteruptAttack)
        (if (or (<= _output_get 0) (<= _output_get_2 0))
          ;[0.15 0.07843 0.1427 0.5] Call Death Delegate
          (Variables|Default|SetIsDead true)
          (Default|CallOnDeath)
          (return true)
          (else
            ;[0.06717 0.07516 0.15 0.5] Call Damage Hit Responses (Knockbacks, slows etc)
            (if true
              (CallFunction|TakeDamageResponse _damageresponseinfo)
              (return true)
              (else
                (Development|PrintString "nO dAMAGE RESPOSNSE")))))))
    (:NoDamage
      (return false))))
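; BP_SpawnMaster coordinates wave-based enemy spawning across linked spawner locations and trigger locations.
; On BeginPlay it registers itself as master with both, and a trigger entry starts the first wave if none is running.
; Each wave tells every spawner to spawn by wave index, while an alive-enemy list tracks additions and deaths.
; When that list empties, it increments the wave and starts the next, with no wave limit here.
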(event Custom|StartWave
  ;[0.05729 0.15 0.03265 0.5] Starting the wave
  (for _array_element (Variables|Default|GetSpawnerLocations)
    (Default|SpawnWave _array_element (Variables|Default|GetCurrentWave))))

(event EventBeginPlay
  ;[0.15 0.00252 0.00947 0.5] Setting up master spawners in enemy spawner locations
  (for _array_element (Variables|Default|GetSpawnerLocations)
    (Default|SetMasterSpawner _array_element self)
    (for _array_element_2 (Variables|Default|GetTriggerLocations)
      (Variables|/Game/Enemies/BP_SpawnTriggerArea.BP_SpawnTriggerArea_C|SetMaster%20Spawner _array_element_2 self))))

(event EventAddEnemyCounttoTotal
  (params (EnemyObject :type BP%20Enemy%20Base%20Object%20Reference))
  ;[0.15 0.15 0.15 0.5] Adding enemies to alive list
  (Utilities|Array|Add (Variables|Default|GetCurrentEnemiesAlive) EnemyObject))

(event EventOnEnemyDeath
  (params (EnemyObject :type BP%20Enemy%20Base%20Object%20Reference))
  (bind _currentenemiesalive (Variables|Default|GetCurrentEnemiesAlive))
  ;[0.15 0.15 0.15 0.5] Removing enemies from alive list and checking to see if we can start the next wave
  (Utilities|Array|RemoveIndex _currentenemiesalive (Utilities|Array|FindItem _currentenemiesalive EnemyObject))
  (if (== (Utilities|Array|Length _currentenemiesalive) 0)
    (Development|PrintString "start next wave")
    (Variables|Default|SetCurrentWave (+ (Variables|Default|GetCurrentWave) 1))
    (CallFunction|StartWave)))

(event EventOnTriggerEnter
  ;[0.15 0 0 0.5] When player enters the room / touches the trigger
  (if (and (== (Variables|Default|GetCurrentWave) 0) (== (Utilities|Array|Length (Variables|Default|GetCurrentEnemiesAlive)) 0))
    (CallFunction|StartWave)))

(fn ConstructionScript)
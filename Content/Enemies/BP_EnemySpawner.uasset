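; Enemy spawner actor that spawns a set number of enemies of a configurable class at its own transform.
; Spawning runs on BeginPlay when SpawnOnStart is set, or whenever OnTrigger fires, with both paths sharing the same logic.
; Each spawned actor is added to CurrentEnemyList, which is then printed to screen as a debug check.
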(event EventBeginPlay
  (bind _spawnamount (Variables|Default|GetSpawnAmount))
  ;[1 0.0215 0.006539 0.5] Events starts here
  (if (Variables|Default|GetSpawnOnStart)
    ;[0.1848 0.6545 0.125 0.5] Spawning Logic
    (if (>= _spawnamount 1)
      (for _index (range 0 (- _spawnamount 1))
        (bind _returnvalue (Game|SpawnActorfromClass (Variables|Default|GetEnemyBlueprintClass) (Transformation|GetActorTransform) "Undefined" "MultiplyWithRoot" 0 0))
        (Utilities|Array|Add (Variables|Default|GetCurrentEnemyList) _returnvalue))
      ;[0.15 0.15 0.15 0.5] printing to know if enemy list array works
      (for (_ _array_index) (Variables|Default|GetCurrentEnemyList)
        (Development|PrintString (Utilities|String|ToString(Integer) _array_index))))))

(event EventOnTrigger
  (bind _spawnamount (Variables|Default|GetSpawnAmount))
  ;[0.1848 0.6545 0.125 0.5] Spawning Logic
  (if (>= _spawnamount 1)
    (for _index (range 0 (- _spawnamount 1))
      (bind _returnvalue (Game|SpawnActorfromClass (Variables|Default|GetEnemyBlueprintClass) (Transformation|GetActorTransform) "Undefined" "MultiplyWithRoot" 0 0))
      (Utilities|Array|Add (Variables|Default|GetCurrentEnemyList) _returnvalue))
    ;[0.15 0.15 0.15 0.5] printing to know if enemy list array works
    (for (_ _array_index) (Variables|Default|GetCurrentEnemyList)
      (Development|PrintString (Utilities|String|ToString(Integer) _array_index)))))

(fn ConstructionScript)
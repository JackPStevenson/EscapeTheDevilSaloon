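; BP_EnemySpawnLocation is a spawn point that spawns the enemies configured for a given wave at its own transform.
; SpawnWave checks that the index exists in WaveInfo, then spawns each entry's enemy type the listed number of times.
; Each spawned enemy receives the MasterSpawner reference and is registered with it for the total enemy count.
; The MasterSpawner reference is supplied through SetMasterSpawner.
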(event EventSpawnWave
  (params (WaveIndex :type Integer))
  (bind _waveinfo (Variables|Default|GetWaveInfo))
  (bind _master_spawner (Variables|Default|GetMaster%20Spawner))
  ;[0.1848 0.6545 0.125 0.5] Spawning Logic
  (if (Utilities|Array|IsValidIndex _waveinfo WaveIndex)
    (for _array_element (Utilities|Struct|BreakS_WaveInfo (Utilities|Array|Get(acopy) _waveinfo WaveIndex))
      (for _index (range 1 (.Amount (Utilities|Struct|BreakS_EnemySpawnInfo _array_element)))
        (bind _returnvalue (Game|SpawnActorfromClass (.EnemyType (Utilities|Struct|BreakS_EnemySpawnInfo _array_element)) (Transformation|GetActorTransform) "Undefined" "MultiplyWithRoot" 0 "/Game/Enemies/KN_Test_Animations/AM_ScuffedPunch.AM_ScuffedPunch" 0))
        (Default|SetMasterSpawner _returnvalue _master_spawner)
        (Default|AddEnemyCounttoTotal _master_spawner _returnvalue)))))

(event EventSetMasterSpawner
  (params (MasterSpawner :type BP%20Spawn%20Master%20Object%20Reference))
  (Variables|Default|SetMaster%20Spawner MasterSpawner))

(fn ConstructionScript)